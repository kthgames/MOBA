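; BP_Dummy is a target dummy for stealth back assassinations by the third-person character.
; An overlap radius shows an assassinate widget while that character is inside, and Tick rotates the widget to face the player camera.
; StealthBackAssassin hides the widget, triggers a delayed switch to ragdoll physics on the mesh, and returns a zeroed reference location and assassin rotation.
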(event OnComponentBeginOverlap(AssassinationRadius)
  (params (OverlappedComponent :type Primitive%20Component%20Object%20Reference) (OtherActor :type Actor%20Object%20Reference) (OtherComp :type Primitive%20Component%20Object%20Reference) (OtherBodyIndex :type Integer) (bFromSweep :type Boolean) (SweepResult :type Hit%20Result%20Structure%20%28by%20ref%29))
  (Utilities|Casting|CastToBP_ThirdPersonCharacter OtherActor)
  (Rendering|SetVisibility (Variables|Default|GetAssassinate%20Widget) true false))

(event OnComponentEndOverlap(AssassinationRadius)
  (params (OverlappedComponent :type Primitive%20Component%20Object%20Reference) (OtherActor :type Actor%20Object%20Reference) (OtherComp :type Primitive%20Component%20Object%20Reference) (OtherBodyIndex :type Integer))
  (Utilities|Casting|CastToBP_ThirdPersonCharacter OtherActor)
  (Rendering|SetVisibility (Variables|Default|GetAssassinate%20Widget) false false))

(event Custom|Ragdoll
  ;[0.07292 0.07292 0.07292] Ragdoll
  (Utilities|FlowControl|Delay 2.5)
  (Physics|SetSimulatePhysics (Variables|Character|GetMesh) true))

(event EventTick
  (params (DeltaSeconds :type Float%20%28single-precision%29))
  (bind _assassinate_widget (Variables|Default|GetAssassinate%20Widget))
  (Transformation|SetWorldRotation _assassinate_widget (Math|Rotator|FindLookatRotation (Transformation|GetWorldLocation _assassinate_widget) (Transformation|GetWorldLocation (Variables|/Script/Engine.PlayerCameraManager|GetTransformComponent (Game|GetPlayerCameraManager 0)))) false false))

(fn ConstructionScript)

(fn StealthBackAssassin
  (CallFunction|Ragdoll)
  (Rendering|SetVisibility (Variables|Default|GetAssassinate%20Widget) false false)
  (return "0, 0, 0" "0, 0, 0"))
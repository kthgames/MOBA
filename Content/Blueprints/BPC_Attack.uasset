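; Attack component for BP_ThirdPersonCharacter that runs a four-step melee combo of sword attacks and a kick.
; IA_Attack, gated by CanAttack, calls SwordAttack, which selects the next attack from AttackIndex.
; Each attack uses a DoOnce and short delay, plays its montage on the character mesh, then advances the index.
; Stopcombo resets the combo state; Swordattackcombo sets IsCombo, which this graph never reads.
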(event Custom|Sword%20Attack
  (if (Variables|Default|Getis%20attacking)
    _
    (else
      (Variables|Default|Setis%20attacking true)))
  (switch int (Variables|Default|Getattack%20index)
    (:0
      (CallFunction|Attack1))
    (:1
      (CallFunction|Attack2))
    (:2
      (CallFunction|Attack3))
    (:3
      (CallFunction|Attack4))))

(event Custom|Stop%20combo
  (Variables|Default|Setis%20attacking false)
  (Variables|Default|Setattack%20index 0)
  (Variables|Default|Setis%20combo%20 false))

(event Custom|Sword%20attack%20combo
  (Variables|Default|Setis%20combo%20 true))

(event Custom|attack%201
  ;[0.07292 0.07292 0.07292] Attack 1
  (Utilities|FlowControl|DoOnce false :!label _label
    (:Completed
      (Utilities|FlowControl|Delay 0.1)
      (Animation|Montage|PlayMontage (Variables|Default|GetCharMesh) "/Game/Characters/RPG_Character/Animations/SwordAttacks/Attack1_Montage.Attack1_Montage"
        (:then
          (Variables|Default|Setattack%20index 1)
          (goto _label Reset))))))

(event Custom|attack%204
  ;[0.07292 0.07292 0.07292] Attack 4
  (Utilities|FlowControl|DoOnce false :!label _label
    (:Completed
      (Utilities|FlowControl|Delay 0.1)
      (Animation|Montage|PlayMontage (Variables|Default|GetCharMesh) "/Game/Characters/RPG_Character/Animations/SwordAttacks/Attack3_Montage.Attack3_Montage"
        (:then
          (Variables|Default|Setattack%20index 4)
          (goto _label Reset))))))

(event Custom|attack%202
  ;[0.07292 0.07292 0.07292] Attack 2
  (Utilities|FlowControl|DoOnce false :!label _label
    (:Completed
      (Utilities|FlowControl|Delay 0.1)
      (Animation|Montage|PlayMontage (Variables|Default|GetCharMesh) "/Game/Characters/RPG_Character/Animations/SwordAttacks/Attack2_Montage.Attack2_Montage"
        (:then
          (Variables|Default|Setattack%20index 2)
          (goto _label Reset))))))

(event Custom|attack%203
  ;[0.07292 0.07292 0.07292] Attack 3
  (Utilities|FlowControl|DoOnce false :!label _label
    (:Completed
      (Utilities|FlowControl|Delay 0.1)
      (Animation|Montage|PlayMontage (Variables|Default|GetCharMesh) "/Game/Characters/RPG_Character/Animations/SwordAttacks/Kick_Montage.Kick_Montage"
        (:then
          (Variables|Default|Setattack%20index 3)
          (goto _label Reset))))))

(event Input|EnhancedActionEvents|EnhancedInputActionIA_Attack
  (params (ActionValue :type Boolean) (ElapsedSeconds :type Float%20%28double-precision%29) (TriggeredSeconds :type Float%20%28double-precision%29) (InputAction :type Input%20Action%20Object%20Reference :default "/Game/ThirdPerson/Input/Actions/IA_Attack.IA_Attack"))
  (:Started
    (if (Variables|Default|Getcan%20attack)
      (CallFunction|SwordAttack))))

(event EventBeginPlay
  (bind _asbp_third_person_character (Utilities|Casting|CastToBP_ThirdPersonCharacter (Components|GetOwner)))
  (Variables|Default|SetCharMesh (Variables|/Script/Engine.Character|GetMesh _asbp_third_person_character)))